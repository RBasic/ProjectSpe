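; Item Blueprint that randomizes its own price, type and stat when play begins.
; Price gets a random value, and a random boolean picks the Type.
; That Type decides the Stat roll, with the true case drawing from a much higher range than the false one.
; The construction script is empty, so every value is set at BeginPlay.
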(event EventBeginPlay
  (Variables|Default|Setprice (+ (Math|Random|RandomInteger 35) 20))
  (bind _output_get (Variables|Default|Settype (Math|Random|RandomBool)))
  (if _output_get
    (Variables|Default|Setstat (+ (Math|Random|RandomInteger 100) 100))
    (else
      (Variables|Default|Setstat (+ (Math|Random|RandomInteger 35) 25)))))

(fn ConstructionScript)