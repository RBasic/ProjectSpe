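; BP_Marchand1 is a merchant actor that shows a shop UI while the third-person character is nearby.
; On BeginPlay it creates the BP_UI widget and spawns three Item actors, storing their references without passing them to the widget.
; Overlapping its Box adds the widget to the viewport and shows the mouse cursor.
; The actor-level end overlap, rather than the Box's, removes the widget and hides the cursor.
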(event OnComponentBeginOverlap(Box)
  (params (OverlappedComponent :type Primitive%20Component%20Object%20Reference) (OtherActor :type Actor%20Object%20Reference) (OtherComp :type Primitive%20Component%20Object%20Reference) (OtherBodyIndex :type Integer) (bFromSweep :type Boolean) (SweepResult :type Hit%20Result%20Structure%20%28by%20ref%29))
  (bind _asbp_third_person_character (Utilities|Casting|CastToBP_ThirdPersonCharacter OtherActor))
  (bind _asplayer_controller (Utilities|Casting|CastToPlayerController (Pawn|GetController _asbp_third_person_character)))
  (UserInterface|Viewport|AddtoViewport (Variables|Default|GetUIShop) 0)
  (Variables|/Script/Engine.PlayerController|SetbShowMouseCursor _asplayer_controller true))

(event EventBeginPlay
  (bind _returnvalue (UserInterface|CreateWidget "/Game/UI/BP_UI.BP_UI_C"))
  (Variables|Default|SetUIShop _returnvalue)
  (bind _returnvalue_2 (Game|SpawnActorfromClass "/Game/Blueprints/Items/Item.Item_C" (Math|Transform|MakeTransform "0, 0, 0" "0, 0, 0" "1.000000,1.000000,1.000000") "Undefined" 0 0))
  (Variables|Default|Setitem_1 _returnvalue_2)
  (bind _returnvalue_3 (Game|SpawnActorfromClass "/Game/Blueprints/Items/Item.Item_C" (Math|Transform|MakeTransform "0, 0, 0" "0, 0, 0" "1.000000,1.000000,1.000000") "Undefined" 0 0))
  (Variables|Default|Setitem_2 _returnvalue_3)
  (bind _returnvalue_4 (Game|SpawnActorfromClass "/Game/Blueprints/Items/Item.Item_C" (Math|Transform|MakeTransform "0, 0, 0" "0, 0, 0" "1.000000,1.000000,1.000000") "Undefined" 0 0))
  (Variables|Default|Setitem_3 _returnvalue_4))

(event Collision|EventActorEndOverlap
  (params (OtherActor :type Actor%20Object%20Reference))
  (bind _asbp_third_person_character (Utilities|Casting|CastToBP_ThirdPersonCharacter OtherActor))
  (bind _asplayer_controller (Utilities|Casting|CastToPlayerController (Pawn|GetController _asbp_third_person_character)))
  (Widget|RemovefromParent (Variables|Default|GetUIShop))
  (Variables|/Script/Engine.PlayerController|SetbShowMouseCursor _asplayer_controller false))

(fn ConstructionScript)