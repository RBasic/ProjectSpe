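; BP_Room is a room actor whose walls can each become a door, configured through the StructDoorActive array.
; Its Construction Script pairs each entry with the child static mesh under Walls at the same index and stores that reference in the struct.
; Entries flagged DoorActive get their wall mesh swapped to DoorMesh.
; The event graph is empty, and an unconnected per-direction door version remains as a fallback.
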(event EventBeginPlay)

(event Collision|EventActorBeginOverlap
  (params (OtherActor :type Actor%20Object%20Reference)))

(event EventTick
  (params (DeltaSeconds :type Float%20%28single-precision%29)))

(fn ConstructionScript
  ;[0.1042 0.1042 0.1042] Activation des portes
  (for (_array_element _array_index) (Variables|Default|GetStruct_DoorActive)
    ;;[0.1527 0.2292 0.2269] Récupère les walls de la scene "Walls"
    (bind _asstatic_mesh_component (Utilities|Casting|CastToStaticMeshComponent (Utilities|Array|Get(acopy) (Components|GetChildrenComponents (Variables|Default|GetWalls) false) _array_index)))
    (Utilities|Array|SetArrayElem (Variables|Default|GetStruct_DoorActive) _array_index (Utilities|Struct|MakeStruct_DoorActive (.dooractive _array_element) _asstatic_mesh_component))
    (if (.dooractive _array_element)
      (Components|StaticMesh|SetStaticMesh (.wall _array_element) (Variables|Default|GetDoorMesh)))))