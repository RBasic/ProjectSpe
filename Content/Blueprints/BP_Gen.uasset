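; Procedural level generator that spawns random room actors and chains them at BoxComponent connectors, up to a room budget.
; LaunchGen clears previous rooms, then GenerateRoom recursively grows from open connectors stored in File; the construction script only cleans.
; Placement reparents components to a random connector, snaps it facing the parent connector, and overlap-tests custom-channel meshes.
; Overlaps retry other connectors, destroying the room when none remain.
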(event EventBeginPlay)

(event Collision|EventActorBeginOverlap
  (params (OtherActor :type Actor%20Object%20Reference)))

(event EventTick
  (params (DeltaSeconds :type Float%20%28single-precision%29)))

(fn ConstructionScript
  (CallFunction|Clean))

(fn GenerateRoom
  (params (ActualNbSalle :type Integer) (Parent :type Scene%20Component%20Object%20Reference))
  (bind _returnvalue (CallFunction|SpawnNewActor))
  (bind _output_get (Variables|Default|SetNewActor _returnvalue))
  (CallFunction|PlaceCorrectly _output_get Parent (Actor|GetComponentsByClass _output_get "/Script/Engine.BoxComponent")))

(fn LaunchGen
  (CallFunction|Clean)
  (CallFunction|GenerateRoom (Variables|Default|GetRoomsToGen) (Variables|Default|GetDefaultSceneRoot)))

(fn Clean
  (for _array_element (Variables|Default|GetRooms)
    (Actor|DestroyActor _array_element))
  (Utilities|Array|Clear (Variables|Default|GetRooms))
  (Utilities|Array|Clear (Variables|Default|GetFile))
  (Variables|Default|SetRoomsToGen (Variables|Default|GetnbSalle)))

(fn VerifOverlaps
  (params (Objet :type Actor%20Object%20Reference))
  (for _array_element (Components|GetChildrenComponents (Variables|/Script/Engine.Actor|GetRootComponent Objet) true)
    (bind _asstatic_mesh_component (Utilities|Casting|CastToStaticMeshComponent _array_element))
    (if (Utilities|Enum|Equal(Enum) (Collision|GetCollisionObjectType _asstatic_mesh_component) "ECC_GameTraceChannel1")
      (bind _outcomponents (Class|KismetSystemLibrary|ComponentOverlapComponents _asstatic_mesh_component (Transformation|GetWorldTransform _asstatic_mesh_component) (Utilities|Array|MakeArray "ObjectTypeQuery7") 0 (Utilities|Array|MakeArray Objet)))
      (if (> (Utilities|Array|Length _outcomponents) 0)
        (Development|PrintString (Utilities|String|Append (Utilities|GetDisplayName (Utilities|Array|Get(acopy) _outcomponents)) (Utilities|GetDisplayName _asstatic_mesh_component)))
        (return (> (Utilities|Array|Length _outcomponents) 0)))))
  (return false))

(fn SelectBox
  (params (TempBoxCollisionArray :type Array%20of%20Box%20Component%20Object%20References))
  (bind _outitem (Utilities|Array|Random TempBoxCollisionArray))
  (if (Utilities|Array|IsEmpty TempBoxCollisionArray)
    (Actor|DestroyActor (Variables|Default|GetNewActor))
    (Development|PrintString "Hello")
    (else
      (Utilities|Array|RemoveItem TempBoxCollisionArray _outitem)
      (return _outitem))))

(fn Rotate
  (params (NewItem :type Actor%20Object%20Reference%20%28by%20ref%29) (CurrentPivot :type Box%20Component%20Object%20Reference) (self3 :type Scene%20Component%20Object%20Reference))
  (bind _output_get (Variables|Default|SetPivotCurrent CurrentPivot))
  (bind _output_get_2 (Variables|Default|SetChildrenArray (Components|GetChildrenComponents (Variables|/Script/Engine.Actor|GetRootComponent NewItem) true)))
  (for _array_element _output_get_2
    (if (!= _array_element _output_get)
      (Transformation|AttachComponentToComponent _array_element _output_get "None" "KeepWorld" "KeepWorld" "KeepWorld" true)))
  (Transformation|SetWorldLocation _output_get (Transformation|GetWorldLocation self3) false false)
  (Transformation|SetWorldRotation _output_get (Math|Rotator|MakeRotator 0.0 0.0 (+ (.yaw (Math|Conversions|RotationFromXVector (Math|Vector|GetForwardVector self3))) 1.8e+02)) false false)
  (return))

(fn SpawnNewActor
  (bind _roomarray (Variables|Default|GetRoomArray))
  (bind _returnvalue (Game|SpawnActorfromClass (Utilities|Array|Get(acopy) _roomarray (Math|Random|RandomInteger (- (Utilities|Array|Length _roomarray) 1))) (Math|Transform|MakeTransform "0, 0, 0" "0, 0, 0" "1.000000,1.000000,1.000000") "Undefined" 0 0))
  (return _returnvalue))

(fn PlaceCorrectly
  (params (self2 :type Actor%20Object%20Reference) (self3 :type Scene%20Component%20Object%20Reference) (TempBoxCollisionArray :type Array%20of%20Box%20Component%20Object%20References))
  (bind _currentpivot (CallFunction|SelectBox TempBoxCollisionArray))
  (CallFunction|Rotate (Variables|Default|GetNewActor) _currentpivot self3)
  (bind _returnvalue (CallFunction|VerifOverlaps (Variables|Default|GetNewActor)))
  (if _returnvalue
    (CallFunction|PlaceCorrectly self2 self3 TempBoxCollisionArray)
    (else
      (for _array_element (Actor|GetComponentsByClass (Variables|Default|GetNewActor) "/Script/Engine.BoxComponent")
        (if (!= _array_element (Variables|Default|GetCurrentPivot))
          (Utilities|Array|Add (Variables|Default|GetFile) _array_element)))
      (Utilities|Array|Add (Variables|Default|GetRooms) (Variables|Default|GetNewActor))
      (for _array_element_2 (Variables|Default|GetFile)
        (Math|Integer|DecrementInt (Variables|Default|GetRoomsToGen)
          (:%20%20
            (if (> (Variables|Default|GetRoomsToGen) 0)
              (Variables|Default|SetNextSpawn _array_element_2)
              (Utilities|Array|RemoveItem (Variables|Default|GetFile) _array_element_2)
              (CallFunction|GenerateRoom (Variables|Default|GetRoomsToGen) (LocalVariables|GetNextSpawn)))))))))